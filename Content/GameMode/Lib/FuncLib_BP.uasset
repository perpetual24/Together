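; Gameplay function library with shared helpers for footsteps, camera tracing and item spawning.
; Footsteps trace downward for the physical material to play a sound, then report tagged AI noise for TempPlayer or Doll, adding camera shake for the player.
; LineTraceCamera returns what lies along the camera's forward vector.
; SpawnItem picks a random point between a component's LL and RH sockets, or a manual location, and spawns with random rotation and Z correction.
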(fn AddFootstepSound
  (params (target :type Actor%20Object%20Reference) (Camera%20Shake :type Camera%20Shake%20Class%20Reference) (Volume :type Float%20%28single-precision%29) (Strength%20Multiply :type Float%20%28single-precision%29))
  (bind _returnvalue (Transformation|GetActorLocation target))
  (bind _returnvalue_2 (Utilities|GetClass target))
  (bind _returnvalue_3 (Transformation|GetActorLocation target))
  (bind _outhit (Collision|LineTraceByChannel 0 _returnvalue_3 (+ _returnvalue_3 "0, 0,-150.000000") "TraceTypeQuery1" false 0 "None"))
  (Class|FuncLib|PlayFootstepSound target (.PhysMat (Collision|BreakHitResult _outhit)) Volume)
  (if (== _returnvalue_2 "/Game/Player/TempPlayer.TempPlayer_C")
    (Class|AISenseHearing|ReportNoiseEvent 0 _returnvalue Strength%20Multiply target 0.0 "PlayerFootstep")
    (Class|PlayerController|ClientPlayCameraShake (Game|GetPlayerController 0) Camera%20Shake 1.2 "CameraLocal" "0, 0, 0")
    (elif (== _returnvalue_2 "/Game/Doll/Doll.Doll_C")
      (Class|AISenseHearing|ReportNoiseEvent 0 _returnvalue Strength%20Multiply target 0.0 "EnermyFootstep"))))

(fn LineTraceCamera
  (params (Trace%20Dist :type Integer) (Camera :type Camera%20Component%20Object%20Reference))
  (bind _returnvalue (Transformation|GetWorldLocation Camera))
  (bind (_outhit _returnvalue_2) (Collision|LineTraceByChannel 0 _returnvalue (+ _returnvalue (* (Math|Vector|GetForwardVector (Transformation|GetWorldRotation Camera)) Trace%20Dist)) "TraceTypeQuery1" false 0 "None"))
  (return _returnvalue_2 (.hitactor _outhit) (.hitcomponent _outhit)))

(fn SpawnItem
  (params (target :type Actor%20Object%20Reference) (Item :type Actor%20Class%20Reference) (Comp :type Primitive%20Component%20Object%20Reference) (Manual%20Location :type Vector))
  (Utilities|IsValid Comp
    (:Is%20Valid
      (bind _returnvalue (Class|FuncLib|RandomVector (Transformation|GetSocketLocation Comp "LL") (Transformation|GetSocketLocation Comp "RH")))
      (bind _returnvalue_2 (Class|FuncLib|RandomRotator "0, 0, 0" "0,180.000000, 0"))
      (bind _returnvalue_3 (Class|FuncLib|SpawnActorwithZCorrection target Item _returnvalue _returnvalue_2))
      (return _returnvalue_3))
    (:Is%20Not%20Valid
      (bind _returnvalue_4 (Class|FuncLib|RandomRotator "0, 0, 0" "0,180.000000, 0"))
      (bind _returnvalue_5 (Class|FuncLib|SpawnActorwithZCorrection target Item Manual%20Location _returnvalue_4))
      (return _returnvalue_5))))