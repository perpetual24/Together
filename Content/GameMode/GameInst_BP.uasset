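; Game instance Blueprint that holds surface data and tracks which area the player and the enemy occupy.
; InitGameInst copies SurfaceDef into the Surface array, calls InitiateAreas and prints a completion message.
; Two notify events store the reported player and enemy areas.
; InitAreaLight looks up actors by dorm hall and stair tags but does nothing with the results, and is not called in these graphs.
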(event Custom|Init%20GameInst
  (CallFunction|InitSurface)
  (Class|GameInst|InitiateAreas)
  (Development|PrintString "Game Inst Init Complete" true true "(R=0.000000,G=0.982576,B=1.000000,A=1.000000)"))

(event EventNotifyEnemyArea
  (params (Area :type Area%20Object%20Reference))
  (Variables|Default|SetEnemyArea Area))

(event EventNotifyPlayerArea
  (params (Area :type Area%20Object%20Reference))
  (Variables|Default|SetPlayerArea Area))

(fn InitSurface
  (for (_array_element _array_index) (Variables|Default|GetSurface_Def)
    (Utilities|Array|SetArrayElem (Variables|Default|GetSurface) _array_index _array_element true)))

(fn InitAreaLight
  (Utilities|FlowControl|Sequence
    (:then_0
      (Actor|GetAllActorswithTag "Dorm_1F_E_Hall"))
    (:then_1
      (Actor|GetAllActorswithTag "Dorm_1F_W_Hall"))
    (:then_2
      (Actor|GetAllActorswithTag "Dorm_1F_Bridge_Hall"))
    (:then_3
      (Actor|GetAllActorswithTag "Dorm_1F_E_Stair"))
    (:then_4
      (Actor|GetAllActorswithTag "Dorm_1F_W_Stair"))
    (:then_5
      (Actor|GetAllActorswithTag "Dorm_2F_W_Hall"))
    (:then_6
      (Actor|GetAllActorswithTag "Dorm_2F_E_Hall"))
    (:then_7
      (Actor|GetAllActorswithTag "Dorm_2F_Bridge_Hall"))))