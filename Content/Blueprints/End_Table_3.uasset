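; End table prop Blueprint with a main body and a drawer, which can host a spawned item.
; On BeginPlay, RandomMaterial picks one of two material variants at random and applies the same one to both meshes.
; The CallSpawnItem event passes the given item to SpawnItem, using the Spawn component as its placement reference.
; The construction script is empty.
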(event EventBeginPlay
  (CallFunction|RandomMaterial))

(event EventCallSpawnItem
  (params (item :type Actor%20Class%20Reference))
  (CallFunction|SpawnItem self item (Variables|Default|GetSpawn) "0, 0, 0"))

(fn ConstructionScript)

(fn RandomMaterial
  (bind _end_table_3_main (Variables|Default|GetEnd_Table_3_Main))
  (bind _end_table_3_drawer (Variables|Default|GetEnd_Table_3_Drawer))
  (switch int (Math|Random|RandomIntegerinRange 0 1)
    (:0
      (Rendering|Material|SetMaterial _end_table_3_main 0 "/Game/Assets/Old_Furnitures_V1/Materials/M_End_Table_3_A.M_End_Table_3_A")
      (Rendering|Material|SetMaterial _end_table_3_drawer 0 "/Game/Assets/Old_Furnitures_V1/Materials/M_End_Table_3_A.M_End_Table_3_A"))
    (:1
      (Rendering|Material|SetMaterial _end_table_3_main 0 "/Game/Assets/Old_Furnitures_V1/Materials/M_End_Table_3_B.M_End_Table_3_B")
      (Rendering|Material|SetMaterial _end_table_3_drawer 0 "/Game/Assets/Old_Furnitures_V1/Materials/M_End_Table_3_B.M_End_Table_3_B"))))