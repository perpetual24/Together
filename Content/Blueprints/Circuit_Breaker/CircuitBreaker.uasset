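; Interactable circuit breaker that the player toggles between on and off by swinging its handle.
; Interact disables interaction and its prompt, then calls TurnOn or TurnOff, which plays or reverses a timeline driving the handle's roll.
; Turning on also emits a short spark burst with random pitch and duration.
; When the timeline finishes, the prompt name follows the IsOff state and interaction is re-enabled.
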(event Custom|Turn%20On
  (Variables|Default|SetisOff false)
  (CallFunction|SpawnSpark)
  (bind _새_트랙_0 (Timeline|타임라인_0 Play)
    (:Update
      (Transformation|SetRelativeRotation (Variables|Default|GetHandle) (Math|Rotator|MakeRotator _새_트랙_0 0.0 0.0) false false))
    (:Finished
      (if (Variables|Default|GetisOff)
        (Variables|Default|SetInteraction%20Name "Turn On")
        (else
          (Variables|Default|SetInteraction%20Name "Turn Off")))
      (CallFunction|EnableInteract)
      (CallFunction|EnableInteractMessageBuild))))

(event Custom|Turn%20Off
  (Variables|Default|SetisOff true)
  (bind _새_트랙_0 (Timeline|타임라인_0 Reverse)
    (:Update
      (Transformation|SetRelativeRotation (Variables|Default|GetHandle) (Math|Rotator|MakeRotator _새_트랙_0 0.0 0.0) false false))
    (:Finished
      (if (Variables|Default|GetisOff)
        (Variables|Default|SetInteraction%20Name "Turn On")
        (else
          (Variables|Default|SetInteraction%20Name "Turn Off")))
      (CallFunction|EnableInteract)
      (CallFunction|EnableInteractMessageBuild))))

(event Custom|Spawn%20Spark
  (bind _returnvalue (Effects|SpawnEmitteratLocation "/Game/Blueprints/Spark/Sparks_Particle.Sparks_Particle" (Transformation|GetWorldLocation (Variables|Default|GetSparkLoc)) (Math|Rotator|MakeRotator 0.0 (Math|Conversions|ToFloat(Integer) (Math|Random|RandomIntegerinRange -180 180)) 0.0)))
  (Utilities|FlowControl|Delay (Math|Random|RandomFloatinRange 0.1 0.2))
  (Components|Activation|Deactivate _returnvalue))

(event EventInteract
  (params (Component :type Primitive%20Component%20Object%20Reference) (isDouble :type Boolean))
  (CallFunction|DisableInteract)
  (CallFunction|DisableInteractMessageBuild)
  (CallFunction|DestroyInteractMessage)
  (if (Variables|Default|GetisOff)
    (CallFunction|Turnon)
    (else
      (CallFunction|TurnOff))))

(fn ConstructionScript)