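; End table prop Blueprint that varies its look and can host a spawned item.
; On BeginPlay it randomly applies one of two end table materials to its mesh.
; The CallSpawnItem event passes the given item and the Spawn component to SpawnItem, which is called on itself but not defined in this graph.
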(event EventBeginPlay
  (CallFunction|RandomMaterial))

(event EventCallSpawnItem
  (params (item :type Actor%20Class%20Reference))
  (CallFunction|SpawnItem self item (Variables|Default|GetSpawn) "0, 0, 0"))

(fn ConstructionScript)

(fn RandomMaterial
  (bind _bp_end_table (Variables|Default|GetBP_End_Table))
  (switch int (Math|Random|RandomIntegerinRange 0 1)
    (:0
      (Rendering|Material|SetMaterial _bp_end_table 0 "/Game/Assets/Old_Furnitures_V1/Materials/M_End_Table_1_A.M_End_Table_1_A"))
    (:1
      (Rendering|Material|SetMaterial _bp_end_table 0 "/Game/Assets/Old_Furnitures_V1/Materials/M_End_Table_1_B.M_End_Table_1_B"))))