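; Interactable single locker whose door opens and closes and which can hold items spawned at three spawn points.
; Interact disables the prompt, swings the door's yaw through timelines behind a gate, then toggles the Open/Close label and re-enables interaction.
; CallSpawnItem routes an item to the spawn component chosen by index.
; BeginPlay randomly applies one of three locker materials to the main mesh.
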(event EventBeginPlay
  (CallFunction|RandomMaterial))

(event Collision|EventActorBeginOverlap
  (params (OtherActor :type Actor%20Object%20Reference)))

(event EventTick
  (params (DeltaSeconds :type Float%20%28single-precision%29))
  (|CallParentFunction DeltaSeconds) ; 지금 이 노드는 비활성 상태입니다. \n핀을 끌어서 다른 노드를 연결하면 활성화됩니다.
)

(event EventInteract
  (params (Component :type Primitive%20Component%20Object%20Reference) (isDouble :type Boolean))
  (bind _door (Variables|Default|GetDoor))
  (CallFunction|DisableInteractMessageBuild)
  (CallFunction|DestroyInteractMessage)
  (CallFunction|DisableInteract)
  (Utilities|FlowControl|Gate false :!label _label
    (:Exit
      (if (Variables|Default|GetisClosed)
        (bind _새_트랙_0 (Timeline|타임라인_0 PlayFromStart)
          (:Update
            (Transformation|SetRelativeRotation _door (Math|Rotator|MakeRotator 0.0 0.0 _새_트랙_0) false false)
            (goto _label Close))
          (:Finished
            (Variables|Default|SetisClosed false)
            (Variables|Default|SetInteraction%20Name "Close")))
        (else
          (bind _새_트랙_0_2 (Timeline|타임라인_1 ReverseFromEnd)
            (:Update
              (Transformation|SetRelativeRotation _door (Math|Rotator|MakeRotator 0.0 0.0 _새_트랙_0_2) false false)
              (goto _label Close))
            (:Finished
              (Variables|Default|SetisClosed true)
              (Variables|Default|SetInteraction%20Name "Open")))))
      (CallFunction|EnableInteract)
      (CallFunction|EnableInteractMessageBuild)
      (goto _label Open))))

(event EventCallSpawnItem
  (params (item :type Actor%20Class%20Reference) (Spawner :type Integer))
  (bind _self self)
  (switch int Spawner
    (:0
      (CallFunction|SpawnItem _self item (Variables|Default|GetSpawn_0) "0, 0, 0"))
    (:1
      (CallFunction|SpawnItem _self item (Variables|Default|GetSpawn_1) "0, 0, 0"))
    (:2
      (CallFunction|SpawnItem _self item (Variables|Default|GetSpawn_2) "0, 0, 0"))))

(fn ConstructionScript
  (|CallParentFunction))

(fn RandomMaterial
  (bind _main (Variables|Default|GetMain))
  (switch int (Math|Random|RandomIntegerinRange 0 2)
    (:0
      (Rendering|Material|SetMaterial _main 0 "/Game/OriginalAssets/Old_Furnitures_V1/Materials/M_Locker_A.M_Locker_A"))
    (:1
      (Rendering|Material|SetMaterial _main 0 "/Game/OriginalAssets/Old_Furnitures_V1/Materials/M_Locker_B.M_Locker_B"))
    (:2
      (Rendering|Material|SetMaterial _main 0 "/Game/OriginalAssets/Old_Furnitures_V1/Materials/M_Locker_C.M_Locker_C"))))