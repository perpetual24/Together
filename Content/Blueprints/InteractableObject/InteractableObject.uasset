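; Base interactable object that shows an on-screen Interaction prompt with a configurable button and action name.
; Continuous calls to ShowInteractMessage create the widget once, and a Tick-driven continuous/off helper removes it through HideInteractMessage when the off event fires.
; An initially open gate lets Enable and Disable events control prompt creation.
; Interact forwards to InteractionEvent, an empty function that serves as the hook for object-specific behavior.
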(event Custom|Hide%20Interact%20Message
  (Utilities|IsValid (Variables|Default|GetInteractionW)
    (:Is%20Valid
      (Default|Destroy (Variables|Default|GetInteractionW))
      (Variables|Default|SetInteractionW 0))))

(event Custom|Disable%20Interact%20Message
  (Utilities|FlowControl|Gate false) ; enters at Close
)

(event Custom|Enable%20Interact%20Message
  (Utilities|FlowControl|Gate false) ; enters at Open
)

(event EventTick
  (params (DeltaSeconds :type Float%20%28single-precision%29))
  (Utilities|ContinuousOffEvent) ; enters at Tick
)

(event EventInteract
  (params (isDouble :type Boolean))
  (CallFunction|InteractionEvent))

(event EventShowInteractMessage
  (Utilities|ContinuousOffEvent
    (:Continuous%20Out
      (Utilities|IsValid (Variables|Default|GetInteractionW)
        (:Is%20Not%20Valid
          (Utilities|FlowControl|Gate false
            (:Exit
              (bind _returnvalue (UserInterface|CreateWidget "/Game/UI/UMG/InGame/Interaction.Interaction_C"))
              (bind _output_get (Variables|Default|SetInteractionW _returnvalue))
              (Default|ConfigText _output_get (Variables|Default|GetButton%20Name) (Variables|Default|GetInteraction%20Name))
              (UserInterface|Viewport|AddtoViewport _output_get 0))))))
    (:Off%20Event
      (CallFunction|HideInteractMessage))))

(fn ConstructionScript)

(fn InteractionEvent
  (return))