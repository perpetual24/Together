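; Interactable locker with left, middle and right doors that the player opens and closes individually.
; InteractionEvent toggles the targeted door and hides the prompt, while per-door timelines drive its yaw.
; InteractMessage allows the prompt only on doors, suppressing it while any busy flag is set.
; The left door clears its flag and re-enables interaction when finished; middle and right also do so on every timeline update.
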(event Custom|InteractMessage
  (if (Math|Boolean|ANDBoolean (!= (Variables|Default|GetComp) (Variables|Default|GetLDoor)) (!= (Variables|Default|GetComp) (Variables|Default|GetMDoor)) (!= (Variables|Default|GetComp) (Variables|Default|GetRDoor)))
    (CallFunction|DisableInteractMessage :!label _label)
    (CallFunction|DisableInteract)
    (CallFunction|HideInteractMessage)
    (elif (Math|Boolean|ORBoolean (Variables|Default|GetisLDoorUpd) (Variables|Default|GetisMDoorUpd) (Variables|Default|GetisRDoorUpd))
      (goto _label)
      (elif (!= (Variables|Default|GetComp) (Variables|Default|GetCabinet))
        (CallFunction|EnableInteractMessage)
        (CallFunction|EnableInteract)))))

(event Custom|Close%20RDoor
  (Variables|Default|SetisRDoorUpd true)
  (bind _rot (Timeline|타임라인_4 PlayFromStart)
    (:Update
      (Transformation|SetRelativeRotation (Variables|Default|GetRDoor) (Math|Rotator|MakeRotator 0.0 0.0 _rot) false false))
    (:Finished
      _))
  (Variables|Default|SetisRDoorClosed true)
  (Variables|Default|SetisRDoorUpd false)
  (CallFunction|EnableInteractMessage)
  (CallFunction|EnableInteract))

(event Custom|Open%20RDoor
  (Variables|Default|SetisRDoorUpd true)
  (bind _rot (Timeline|타임라인_5 PlayFromStart)
    (:Update
      (Transformation|SetRelativeRotation (Variables|Default|GetRDoor) (Math|Rotator|MakeRotator 0.0 0.0 _rot) false false))
    (:Finished
      _))
  (Variables|Default|SetisRDoorClosed false)
  (Variables|Default|SetisRDoorUpd false)
  (CallFunction|EnableInteractMessage)
  (CallFunction|EnableInteract))

(event Custom|Open%20LDoor
  (Variables|Default|SetisLDoorUpd true)
  (bind _rot (Timeline|타임라인_0 PlayFromStart)
    (:Update
      (Transformation|SetRelativeRotation (Variables|Default|GetLDoor) (Math|Rotator|MakeRotator 0.0 0.0 _rot) false false))
    (:Finished
      (Variables|Default|SetisLDoorClosed false)
      (Variables|Default|SetisLDoorUpd false)
      (CallFunction|EnableInteractMessage)
      (CallFunction|EnableInteract))))

(event Custom|Close%20LDoor
  (Variables|Default|SetisLDoorUpd true)
  (bind _rot (Timeline|타임라인_1 PlayFromStart)
    (:Update
      (Transformation|SetRelativeRotation (Variables|Default|GetLDoor) (Math|Rotator|MakeRotator 0.0 0.0 _rot) false false))
    (:Finished
      (Variables|Default|SetisLDoorClosed true)
      (Variables|Default|SetisLDoorUpd false)
      (CallFunction|EnableInteractMessage)
      (CallFunction|EnableInteract))))

(event Custom|Close%20MDoor
  (Variables|Default|SetisMDoorUpd true)
  (bind _rot (Timeline|타임라인_3 PlayFromStart)
    (:Update
      (Transformation|SetRelativeRotation (Variables|Default|GetMDoor) (Math|Rotator|MakeRotator 0.0 0.0 _rot) false false))
    (:Finished
      _))
  (Variables|Default|SetisMDoorClosed true)
  (Variables|Default|SetisMDoorUpd false)
  (CallFunction|EnableInteractMessage)
  (CallFunction|EnableInteract))

(event Custom|Open%20MDoor
  (Variables|Default|SetisMDoorUpd true)
  (bind _rot (Timeline|타임라인_2 PlayFromStart)
    (:Update
      (Transformation|SetRelativeRotation (Variables|Default|GetMDoor) (Math|Rotator|MakeRotator 0.0 0.0 _rot) false false))
    (:Finished
      _))
  (Variables|Default|SetisMDoorClosed false)
  (Variables|Default|SetisMDoorUpd false)
  (CallFunction|EnableInteractMessage)
  (CallFunction|EnableInteract))

(fn ConstructionScript)

(fn InteractionEvent
  (params (Component :type Primitive%20Component%20Object%20Reference))
  (|CallParentFunction Component)
  (if (and (not (Variables|Default|GetisLDoorUpd)) (== Component (Variables|Default|GetLDoor)))
    (if (Variables|Default|GetisLDoorClosed)
      (CallFunction|OpenLDoor)
      (CallFunction|DisableInteract)
      (CallFunction|HideInteractMessage)
      (CallFunction|DisableInteractMessage)
      (else
        (CallFunction|CloseLDoor)
        (CallFunction|DisableInteract)
        (CallFunction|HideInteractMessage)
        (CallFunction|DisableInteractMessage)))
    (elif (and (not (Variables|Default|GetisMDoorUpd)) (== Component (Variables|Default|GetMDoor)))
      (if (Variables|Default|GetisMDoorClosed)
        (CallFunction|OpenMDoor)
        (CallFunction|DisableInteract)
        (CallFunction|HideInteractMessage)
        (CallFunction|DisableInteractMessage)
        (else
          (CallFunction|CloseMDoor)
          (CallFunction|DisableInteract)
          (CallFunction|HideInteractMessage)
          (CallFunction|DisableInteractMessage)))
      (elif (and (not (Variables|Default|GetisRDoorUpd)) (== Component (Variables|Default|GetRDoor)))
        (if (Variables|Default|GetisRDoorClosed)
          (CallFunction|OpenRDoor)
          (CallFunction|DisableInteract)
          (CallFunction|HideInteractMessage)
          (CallFunction|DisableInteractMessage)
          (else
            (CallFunction|CloseRDoor)
            (CallFunction|DisableInteract)
            (CallFunction|HideInteractMessage)
            (CallFunction|DisableInteractMessage)))))))

(fn InteractMessageAppear
  (|CallParentFunction)
  (CallFunction|InteractMessage))