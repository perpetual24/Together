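; Area volume actor that reports to the game instance when the player (TempPlayer) or enemy (Doll) is inside it.
; A collision overlap event and a once-per-second tick both feed a shared notify function, which matches the exact actor class and sends a player or enemy area message.
; The periodic check only notifies when exactly one actor of that class overlaps.
; The construction script sets the area's enum from an instance variable.
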(event OnComponentBeginOverlap(CollisionComponent)
  (params (OverlappedComponent :type Primitive%20Component%20Object%20Reference) (OtherActor :type Actor%20Object%20Reference) (OtherComp :type Primitive%20Component%20Object%20Reference) (OtherBodyIndex :type Integer) (bFromSweep :type Boolean) (SweepResult :type Hit%20Result%20Structure%20%28by%20ref%29))
  (CallFunction|NotifyPlayerorEnemyArea OtherActor "/Game/Player/TempPlayer.TempPlayer_C" "/Game/Doll/Doll.Doll_C"))

(event EventTick
  (params (DeltaSeconds :type Float%20%28single-precision%29))
  (Utilities|FlowControl|Sequence
    (:then_0
      (CallFunction|CheckEnemyOverlapping))
    (:then_1
      (CallFunction|CheckPlayerOverlapping))))

(event EventBeginPlay
  (Actor|Tick|SetActorTickInterval 1.0))

(fn ConstructionScript
  (Variables|Default|SetAreaEnum (Variables|Default|GetAreaEnum_Inst)))

(fn NotifyPlayerorEnemyArea
  (params (Actor :type Object%20Object%20Reference) (Player%20Class :type Object%20Class%20Reference) (Enemy%20Class :type Object%20Class%20Reference))
  (bind _returnvalue (Game|GetGameInstance))
  (bind _returnvalue_2 (Utilities|GetClass Actor))
  (bind _self self)
  (if (== _returnvalue_2 Player%20Class)
    (Class|AreaInterface|NotifyPlayerArea(Message) _returnvalue _self)
    (elif (== _returnvalue_2 Enemy%20Class)
      (Class|AreaInterface|NotifyEnemyArea(Message) _returnvalue _self))))

(fn CheckEnemyOverlapping
  (bind _overlappingactors (Collision|GetOverlappingActors "/Game/Doll/Doll.Doll_C" :!class /Script/Engine.Actor))
  (if (== (Utilities|Array|Length _overlappingactors) 1)
    (CallFunction|NotifyPlayerorEnemyArea (Utilities|Array|Get(acopy) _overlappingactors) "/Game/Player/TempPlayer.TempPlayer_C" "/Game/Doll/Doll.Doll_C")))

(fn CheckPlayerOverlapping
  (bind _overlappingactors (Collision|GetOverlappingActors "/Game/Player/TempPlayer.TempPlayer_C" :!class /Script/Engine.Actor))
  (if (== (Utilities|Array|Length _overlappingactors) 1)
    (CallFunction|NotifyPlayerorEnemyArea (Utilities|Array|Get(acopy) _overlappingactors) "/Game/Player/TempPlayer.TempPlayer_C" "/Game/Doll/Doll.Doll_C")))