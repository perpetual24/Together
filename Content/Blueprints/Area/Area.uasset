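; Area trigger actor that reports when the player or an enemy enters it.
; On begin overlap of its collision component, it checks the other actor's exact class against TempPlayer (player) and Doll (enemy).
; A match sends the Area value to the game instance through the corresponding player or enemy area message; other actors are ignored.
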(event OnComponentBeginOverlap(CollisionComponent)
  (params (OverlappedComponent :type Primitive%20Component%20Object%20Reference) (OtherActor :type Actor%20Object%20Reference) (OtherComp :type Primitive%20Component%20Object%20Reference) (OtherBodyIndex :type Integer) (bFromSweep :type Boolean) (SweepResult :type Hit%20Result%20Structure%20%28by%20ref%29))
  (CallFunction|NotifyPlayerorEnermyArea OtherActor "/Game/Player/TempPlayer.TempPlayer_C" "/Game/Doll/Doll.Doll_C"))

(fn ConstructionScript)

(fn NotifyPlayerorEnermyArea
  (params (Actor :type Actor%20Object%20Reference) (PlayerClass :type Actor%20Class%20Reference) (EnermyClass :type Actor%20Class%20Reference))
  (bind _returnvalue (Game|GetGameInstance))
  (bind _returnvalue_2 (Utilities|GetClass Actor))
  (bind _area (Variables|Default|GetArea))
  (if (== _returnvalue_2 PlayerClass)
    (Class|AreaInterface|NotifyPlayerArea(Message) _returnvalue _area)
    (elif (== _returnvalue_2 EnermyClass)
      (Class|AreaInterface|NotifyEnermyArea(Message) _returnvalue _area))))