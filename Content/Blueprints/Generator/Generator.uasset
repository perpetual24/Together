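; Generator actor with start and stop engine events that play startup, looping and shutdown sounds and shake its body mesh.
; Timelines ramp Power, which shortens the actor's tick interval as it rises.
; While running, a gate on Tick offsets the mesh's world Y from its BeginPlay position using a sine of delta time and that interval.
; Tick also switches to the loop sound once the start sound finishes, guarded by a DoOnce that stopping resets.
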(event Custom|Start%20Engine
  (Utilities|FlowControl|Sequence
    (:then_0
      (bind _새_트랙_0 (Timeline|타임라인_0 PlayFromStart)
        (:Update
          (Variables|Default|Setpower _새_트랙_0))))
    (:then_1
      (Audio|Components|Audio|Play (Variables|Default|GetGenerator_Sound) 0.0)
      (Variables|Default|SetisOn true)
      (CallFunction|BrizStart))))

(event Custom|Stop%20Engine
  (bind _generator_sound (Variables|Default|GetGenerator_Sound))
  (bind _generator_sound_2 (Variables|Default|GetGenerator_Sound))
  (Utilities|FlowControl|Sequence
    (:then_0
      (bind _새_트랙_0 (Timeline|타임라인_1 ReverseFromEnd)
        (:Update
          (Variables|Default|Setpower _새_트랙_0))))
    (:then_1
      (Audio|Components|Audio|SetSound _generator_sound "/Game/Generator_SoundEnd.Generator_SoundEnd")
      (Audio|Components|Audio|Play _generator_sound 0.0)
      (Variables|Default|SetisOn false)
      (CallFunction|BrizEnd)
      (Utilities|FlowControl|DoOnce false) ; enters at Reset
    )))

(event Custom|Briz
  (Transformation|SetWorldLocation (Variables|Default|Getuntitled_defaultMaterial_004) (Math|Vector|MakeVector (Variables|Default|Getorigin_x) (|((3*(sin((b*x))))+a) (Variables|Default|Getorigin_y) (Utilities|Time|GetWorldDeltaSeconds) (|2*pi/a 3.14 (+ (* (Variables|Default|Getpower) -0.49) 0.5))) (Variables|Default|Getorigin_z)) false false))

(event Custom|Briz%20End
  (Utilities|FlowControl|Gate true) ; enters at Close
)

(event Custom|Briz%20Start
  (Utilities|FlowControl|Gate true) ; enters at Open
)

(event EventTick
  (params (DeltaSeconds :type Float%20%28single-precision%29))
  (bind _generator_sound (Variables|Default|GetGenerator_Sound))
  (Actor|Tick|SetActorTickInterval (+ (* (Variables|Default|Getpower) -0.49) 0.5))
  (Utilities|FlowControl|Sequence
    (:then_0
      (Utilities|FlowControl|Gate true
        (:Exit
          (CallFunction|Briz))))
    (:then_1
      (if (and (Variables|Default|GetisOn) (not (Audio|Components|Audio|IsPlaying (Variables|Default|GetGenerator_Sound))))
        (Utilities|FlowControl|DoOnce false
          (:Completed
            (Audio|Components|Audio|SetSound _generator_sound "/Game/Generator_SoundLoop.Generator_SoundLoop")
            (Audio|Components|Audio|Play _generator_sound 0.0)))))))

(event EventBeginPlay
  (bind _untitled_defaultmaterial_004 (Variables|Default|Getuntitled_defaultMaterial_004))
  (bind _returnvalue (Transformation|GetWorldLocation _untitled_defaultmaterial_004))
  (Variables|Default|Setorigin_y (.y _returnvalue))
  (Variables|Default|Setorigin_x (.x _returnvalue))
  (Variables|Default|Setorigin_z (.z _returnvalue)))

(fn ConstructionScript)