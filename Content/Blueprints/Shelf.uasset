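; Shelf Blueprint that places an item at one of eight positions on the shelf.
; The CallSpawnItem event picks a random slot and passes the item with that slot's component (left or right, numbered 1 to 4) to SpawnItem.
; The event does no check for occupied slots, and the construction script is empty.
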(event EventCallSpawnItem
  (params (item :type Actor%20Class%20Reference))
  (bind _self self)
  (switch int (Math|Random|RandomIntegerinRange 0 7)
    (:0
      (CallFunction|SpawnItem _self item (Variables|Default|Get1_L) "0, 0, 0"))
    (:1
      (CallFunction|SpawnItem _self item (Variables|Default|Get1_R) "0, 0, 0"))
    (:2
      (CallFunction|SpawnItem _self item (Variables|Default|Get2_R) "0, 0, 0"))
    (:3
      (CallFunction|SpawnItem _self item (Variables|Default|Get3_L) "0, 0, 0"))
    (:4
      (CallFunction|SpawnItem _self item (Variables|Default|Get3_R) "0, 0, 0"))
    (:5
      (CallFunction|SpawnItem _self item (Variables|Default|Get4_L) "0, 0,0.000000"))
    (:6
      (CallFunction|SpawnItem _self item (Variables|Default|Get4_R) "0, 0, 0"))
    (:7
      (CallFunction|SpawnItem _self item (Variables|Default|Get2_L) "0, 0, 0"))))

(fn ConstructionScript)