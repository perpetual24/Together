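; Enterable file cabinet with double doors that the player can open, close and peek out of from inside.
; Interaction toggles both doors through mirrored yaw timelines, with a gate and interact disabling blocking re-triggers mid-animation.
; A box trigger tracks whether the player is inside, enabling the LM interaction to peek.
; A continuous-to-press/release helper, polled on Tick, turns that held input into one door swinging out and reversing on release.
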(event OnComponentBeginOverlap(Box5)
  (params (OverlappedComponent :type Primitive%20Component%20Object%20Reference) (OtherActor :type Actor%20Object%20Reference) (OtherComp :type Primitive%20Component%20Object%20Reference) (OtherBodyIndex :type Integer) (bFromSweep :type Boolean) (SweepResult :type Hit%20Result%20Structure%20%28by%20ref%29))
  (if (== OtherActor (Game|Player|GetPlayerPawn 0))
    (Variables|Default|SetisPlayerInside true)))

(event OnComponentEndOverlap(Box5)
  (params (OverlappedComponent :type Primitive%20Component%20Object%20Reference) (OtherActor :type Actor%20Object%20Reference) (OtherComp :type Primitive%20Component%20Object%20Reference) (OtherBodyIndex :type Integer))
  (if (== OtherActor (Game|Player|GetPlayerPawn 0))
    (Variables|Default|SetisPlayerInside false)))

(event Custom|Door%20Interact
  (CallFunction|DisableInteractMessageBuild)
  (CallFunction|DestroyInteractMessage)
  (CallFunction|DisableInteract)
  (Utilities|FlowControl|Gate false :!label _label
    (:Exit
      (if (Variables|Default|GetisDoorClosed)
        (bind _새_트랙_2 (Timeline|타임라인_2 PlayFromStart)
          (:Update
            (Transformation|SetRelativeRotation (Variables|Default|GetSM_File_Cabinet_Main1) (Math|Rotator|MakeRotator 0.0 0.0 _새_트랙_2) false false)
            (Transformation|SetRelativeRotation (Variables|Default|GetSM_File_Cabinet_Main) (Math|Rotator|MakeRotator 0.0 0.0 (* -1 _새_트랙_2)) false false)
            (goto _label Close))
          (:Finished
            (Variables|Default|SetisDoorClosed false)
            (Variables|Default|SetInteraction%20Name "Close")))
        (else
          (bind _새_트랙_2_2 (Timeline|타임라인_3 ReverseFromEnd)
            (:Update
              (Transformation|SetRelativeRotation (Variables|Default|GetSM_File_Cabinet_Main1) (Math|Rotator|MakeRotator 0.0 0.0 _새_트랙_2_2) false false)
              (Transformation|SetRelativeRotation (Variables|Default|GetSM_File_Cabinet_Main) (Math|Rotator|MakeRotator 0.0 0.0 (* -1 _새_트랙_2_2)) false false)
              (goto _label Close))
            (:Finished
              (Variables|Default|SetisDoorClosed true)
              (Variables|Default|SetInteraction%20Name "Open")))))
      (CallFunction|EnableInteract)
      (CallFunction|EnableInteractMessageBuild)
      (goto _label Open))))

(event Custom|Peek
  (if (Variables|Default|GetisPlayerInside)
    (Utilities|ContinuoustoPressRelease
      (:Press
        (CallFunction|DisableInteractMessageBuild)
        (CallFunction|DestroyInteractMessage)
        (Variables|Default|SetisDoorClosed_Peek false)
        (bind _새_트랙_0 (Timeline|타임라인_1 Play)
          (:Update
            (Transformation|SetRelativeRotation (Variables|Default|GetSM_File_Cabinet_Main1) (Math|Rotator|MakeRotator 0.0 0.0 _새_트랙_0) false false))
          (:Finished
            (CallFunction|EnableInteractMessageBuild))))
      (:Release
        (CallFunction|DisableInteractMessageBuild)
        (CallFunction|DestroyInteractMessage)
        (Variables|Default|SetisDoorClosed_Peek true)
        (Timeline|타임라인_1 Reverse)))))

(event EventBeginPlay)

(event Collision|EventActorBeginOverlap
  (params (OtherActor :type Actor%20Object%20Reference)))

(event EventTick
  (params (DeltaSeconds :type Float%20%28single-precision%29))
  (|CallParentFunction DeltaSeconds)
  (Utilities|ContinuoustoPressRelease) ; enters at Tick
)

(fn ConstructionScript
  (|CallParentFunction))

(fn InteractionEvent
  (params (Component :type Primitive%20Component%20Object%20Reference))
  (|CallParentFunction 0)
  (CallFunction|DoorInteract))

(fn InteractionEventLM
  (|CallParentFunction)
  (CallFunction|Peek))