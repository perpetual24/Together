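; Broken light fixture that flickers in random bursts, toggling two bulb materials, a rect light's intensity and audio.
; Tick drives nested gates and random delays to time each Blink burst, with a small chance of going dark afterward.
; Sparks fire rarely on Tick or randomly on switch-off, when audio also cuts.
; Separate events enable or disable blinking and switch the light on or off by area.
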(event Custom|Turn%20Out
  (CallFunction|TurnOffLight)
  (Utilities|FlowControl|Gate false) ; enters at Close
)

(event Custom|Spawn%20Sparks
  (bind _returnvalue (Effects|SpawnEmitteratLocation "/Game/Blueprints/Spark/Sparks_Particle.Sparks_Particle" (Transformation|GetWorldLocation (Variables|Default|GetParticleLoc)) (Math|Rotator|MakeRotator 0.0 0.0 (Math|Conversions|ToFloat(Integer) (Math|Random|RandomIntegerinRange -180 180)))))
  (Utilities|FlowControl|Delay (Math|Random|RandomFloatinRange 0.1 0.2))
  (Components|Activation|Deactivate _returnvalue))

(event Custom|Blink
  (Utilities|FlowControl|DoOnce false :!label _label
    (:Completed
      (CallFunction|TurnOffLight)
      (Utilities|FlowControl|Delay (Math|Random|RandomFloatinRange 0.2 0.3))
      (CallFunction|TurnonLight)
      (goto _label Reset))))

(event Custom|Disable%20Blinking
  (CallFunction|TurnonLight)
  (Utilities|FlowControl|Gate false) ; enters at Close
)

(event Custom|Enable%20Blinking
  (Utilities|FlowControl|Gate false) ; enters at Open
)

(event EventTick
  (params (DeltaSeconds :type Float%20%28single-precision%29))
  (if (== 1 (Math|Random|RandomIntegerinRange 1 10000))
    (CallFunction|SpawnSparks))
  (Utilities|FlowControl|Gate false
    (:Exit
      (Utilities|FlowControl|Sequence
        (:then_0
          (Utilities|FlowControl|Gate true :!label _label
            (:Exit
              (CallFunction|Blink))))
        (:then_1
          (Utilities|FlowControl|Delay (Math|Random|RandomFloatinRange 3.0 1e+01))
          (Utilities|FlowControl|Sequence
            (:then_0
              (goto _label Open))
            (:then_1
              (Utilities|FlowControl|Delay (Math|Random|RandomFloatinRange 1.0 1.2))
              (Utilities|FlowControl|Sequence
                (:then_0
                  (goto _label Close))
                (:then_1
                  (if (== 1 (Math|Random|RandomIntegerinRange 1 100))
                    (CallFunction|TurnOut)))))))))))

(event EventTurnOffLightArea
  (CallFunction|TurnOffLight)
  (Utilities|FlowControl|Gate false) ; enters at Close
)

(event EventTurnonLightArea
  (CallFunction|TurnonLight)
  (Utilities|FlowControl|Gate false) ; enters at Open
)

(fn ConstructionScript)

(fn TurnOffLight
  (Rendering|Material|SetMaterial (Variables|Default|GetLight1) 0 "/Game/OriginalAssets/AbandonedBuilding/Materials/Props/MI_Prop_LighBulb001a_Off.MI_Prop_LighBulb001a_Off")
  (Rendering|Material|SetMaterial (Variables|Default|GetLight2) 0 "/Game/OriginalAssets/AbandonedBuilding/Materials/Props/MI_Prop_LighBulb001a_Off.MI_Prop_LighBulb001a_Off")
  (Rendering|Components|Light|SetIntensity (Variables|Default|GetRectLight) 0.0)
  (if (Math|Random|RandomBool)
    (CallFunction|SpawnSparks)
    (Components|Activation|Deactivate (Variables|Default|GetAudio))))

(fn TurnonLight
  (Rendering|Material|SetMaterial (Variables|Default|GetLight1) 0 "/Game/OriginalAssets/AbandonedBuilding/Materials/Props/MI_Prop_LighBulb001a_ON.MI_Prop_LighBulb001a_ON")
  (Rendering|Material|SetMaterial (Variables|Default|GetLight2) 0 "/Game/OriginalAssets/AbandonedBuilding/Materials/Props/MI_Prop_LighBulb001a_ON.MI_Prop_LighBulb001a_ON")
  (Rendering|Components|Light|SetIntensity (Variables|Default|GetRectLight) 10680.87793)
  (Components|Activation|Activate (Variables|Default|GetAudio) false))