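; Interactable bunker door that opens and closes with an animated opening mechanism.
; Interact disables interaction and its prompt, then starts opening or closing based on IsClosed.
; Two timelines chain: opener parts roll, then after a short delay the door and hinges yaw, with closing running in reverse order.
; ExecuteOpen and ExecuteClose flags steer the shared Finished callbacks, which restore interaction and update the prompt name when motion ends.
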(event Custom|Open%20Door
  (Variables|Default|SetExecuteOpen true)
  (bind _새_트랙_0 (Timeline|Opener%20Open Play)
    (:Update
      (Transformation|SetRelativeRotation (Variables|Default|GetOpener_F) (Math|Rotator|MakeRotator _새_트랙_0 0.0 0.0) false false)
      (Transformation|SetRelativeRotation (Variables|Default|GetOpener_B) (Math|Rotator|MakeRotator _새_트랙_0 0.0 1.8e+02) false false))
    (:Finished
      (CallFunction|CloseDoorEnd)
      (Utilities|FlowControl|Delay 0.5)
      (if (Variables|Default|GetExecuteOpen)
        (bind _새_트랙_0_2 (Timeline|Door%20Open Play)
          (:Update
            (Transformation|SetRelativeRotation (Variables|Default|GetDoor) (Math|Rotator|MakeRotator 0.0 0.0 _새_트랙_0_2) false false)
            (Transformation|SetRelativeRotation (Variables|Default|GetHinge_Up) (Math|Rotator|MakeRotator 0.0 0.0 _새_트랙_0_2) false false)
            (Transformation|SetRelativeRotation (Variables|Default|GetHinge_Down) (Math|Rotator|MakeRotator 0.0 0.0 _새_트랙_0_2) false false))
          (:Finished
            (CallFunction|OpenDoorEnd)
            (if (Variables|Default|GetExecuteClose)
              (Timeline|Opener%20Open Reverse))))))))

(event Custom|Close%20Door
  (Variables|Default|SetExecuteClose true)
  (bind _새_트랙_0 (Timeline|Door%20Open Reverse)
    (:Update
      (Transformation|SetRelativeRotation (Variables|Default|GetDoor) (Math|Rotator|MakeRotator 0.0 0.0 _새_트랙_0) false false)
      (Transformation|SetRelativeRotation (Variables|Default|GetHinge_Up) (Math|Rotator|MakeRotator 0.0 0.0 _새_트랙_0) false false)
      (Transformation|SetRelativeRotation (Variables|Default|GetHinge_Down) (Math|Rotator|MakeRotator 0.0 0.0 _새_트랙_0) false false))
    (:Finished
      (CallFunction|OpenDoorEnd)
      (if (Variables|Default|GetExecuteClose)
        (bind _새_트랙_0_2 (Timeline|Opener%20Open Reverse)
          (:Update
            (Transformation|SetRelativeRotation (Variables|Default|GetOpener_F) (Math|Rotator|MakeRotator _새_트랙_0_2 0.0 0.0) false false)
            (Transformation|SetRelativeRotation (Variables|Default|GetOpener_B) (Math|Rotator|MakeRotator _새_트랙_0_2 0.0 1.8e+02) false false))
          (:Finished
            (CallFunction|CloseDoorEnd)
            (Utilities|FlowControl|Delay 0.5)
            (if (Variables|Default|GetExecuteOpen)
              (Timeline|Door%20Open Play))))))))

(event Custom|Open%20Door%20End
  (Variables|Default|SetExecuteOpen false)
  (Variables|Default|SetisClosed false)
  (if (not (Variables|Default|GetExecuteClose))
    (Variables|Default|SetInteraction%20Name "Close Door")
    (CallFunction|EnableInteract)
    (CallFunction|EnableInteractMessageBuild)))

(event Custom|Close%20Door%20End
  (Variables|Default|SetExecuteClose false)
  (Variables|Default|SetisClosed true)
  (if (not (Variables|Default|GetExecuteOpen))
    (Variables|Default|SetInteraction%20Name "Open Door")
    (CallFunction|EnableInteract)
    (CallFunction|EnableInteractMessageBuild)))

(event EventInteract
  (params (Component :type Primitive%20Component%20Object%20Reference) (isDouble :type Boolean))
  (CallFunction|DisableInteractMessageBuild)
  (CallFunction|DisableInteract)
  (CallFunction|DestroyInteractMessage)
  (if (Variables|Default|GetisClosed)
    (CallFunction|OpenDoor)
    (else
      (CallFunction|CloseDoor))))

(fn ConstructionScript)